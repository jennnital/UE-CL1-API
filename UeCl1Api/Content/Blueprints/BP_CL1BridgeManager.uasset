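; Debug manager actor that exercises the CL1 bridge subsystem from keyboard input, printing results to screen.
; BeginPlay opens the subsystem's receiver on all interfaces, and key 1 prints per-channel rates from it.
; Keys 2 and 3 point the control target at localhost on a separate port, then send a single stimulation from variables or a grouped, non-interrupting stim plan.
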(event EventBeginPlay
  (Class|Cl1BridgeSubsystem|StartReceiver (Subsystems|GetCl1BridgeSubsystem) 12345 "0.0.0.0")
  (Development|PrintString "CL1 Receiver Open"))

(event Input|KeyboardEvents|1
  (params (Key :type Key%20Structure :default "None"))
  (:Pressed
    (for _array_element (Class|Cl1BridgeSubsystem|GetChannelRates (Subsystems|GetCl1BridgeSubsystem) 1.0)
      (Development|PrintString (Utilities|String|Append "Channel:" (Utilities|String|ToString(Integer) (.Channel (Utilities|Struct|BreakCl1ChannelRate _array_element))) ", Rate:" (Utilities|String|ToString(Float) (.RateHz (Utilities|Struct|BreakCl1ChannelRate _array_element))))))))

(event Input|KeyboardEvents|3
  (params (Key :type Key%20Structure :default "None"))
  (bind _returnvalue (Subsystems|GetCl1BridgeSubsystem))
  (:Pressed
    (Class|Cl1BridgeSubsystem|ConfigureControlTarget _returnvalue "127.0.0.1" 12346)
    (bind _outdescription (Class|Cl1BridgeSubsystem|SendStimPlan _returnvalue (Utilities|Array|MakeArray (Utilities|Struct|MakeCl1StimPlanGroup) (Utilities|Struct|MakeCl1StimPlanGroup) "") false))
    (Development|PrintString _outdescription)))

(event Input|KeyboardEvents|2
  (params (Key :type Key%20Structure :default "None"))
  (bind _returnvalue (Subsystems|GetCl1BridgeSubsystem))
  (:Pressed
    (Class|Cl1BridgeSubsystem|ConfigureControlTarget _returnvalue "127.0.0.1" 12346)
    (bind (_outchannels _outfreqhz _outpulsewidth _outamplitude _outduration _returnvalue_2) (Class|Cl1BridgeSubsystem|SendStimulation _returnvalue (Variables|Default|GetChannels) (Variables|Default|GetFreq%20Hz) (Variables|Default|GetPulse%20Width%20Us) (Variables|Default|GetAmplitude%20Ua) (Variables|Default|GetDuration%20Ms) false))
    (Development|PrintString (Utilities|String|Append "Sending Stim:" (Utilities|String|ToString(Boolean) _returnvalue_2) ", Channels: " _outchannels))))

(fn ConstructionScript)